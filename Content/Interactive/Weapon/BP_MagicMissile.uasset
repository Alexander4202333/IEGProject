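; BP_MagicMissile is a weapon actor for a magic attack that damages enemies and rewards the player with energy.
; On spawn it sets a short life span and plays a non-spatial fireball sound.
; When DamageComponent overlaps a BPEnemy, it applies MagicDamge with the player character as damage causer, then calls AddEnergy on that player.
; The overlap does not destroy the missile, so it persists until its life span expires.
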(event `self.ReceiveBeginPlay`
  (`self.SetLifeSpan` 6.0)
  (`GameplayStatics.PlaySound2D` "/Game/Sound/Magic/fireball4.fireball4" 1.0 1.0 0.0 null null))

(event `self.DamageComponent.OnComponentBeginOverlap`
  (params (OverlappedComponent :type "PrimitiveComponent Object Reference") (OtherActor :type "Actor Object Reference") (OtherComp :type "PrimitiveComponent Object Reference") (OtherBodyIndex :type Integer) (bFromSweep :type Boolean) (SweepResult :type "HitResult Structure (by ref)"))
  (bind _asbpenemy (cast `/Game/Character/BPEnemy` OtherActor))
  (bind _asbp_my_main_char (cast `/Game/Character/BP_MyMainChar` (`GameplayStatics.GetPlayerPawn` 0)))
  (`GameplayStatics.ApplyDamage` _asbpenemy (`self.MagicDamge`) null _asbp_my_main_char)
  (bind _asbp_my_main_char_2 (cast `/Game/Character/BP_MyMainChar` (`GameplayStatics.GetPlayerPawn` 0)))
  (`MyMainChar.AddEnergy` _asbp_my_main_char_2 4.0))

(fn `UserConstructionScript`)