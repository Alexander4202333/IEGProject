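; Enemy magic missile projectile that damages the player character or is absorbed by the shield skill.
; On BeginPlay it caps its projectile speed and sets a limited lifespan.
; Overlaps on its damage component either hit a shield, playing a heal sound and granting the player energy, or hit the player's capsule and apply magic damage.
; Either outcome shortens the lifespan so the missile disappears almost immediately.
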(event `self.ReceiveBeginPlay`
  (set `ProjectileMovementComponent.MaxSpeed` 400.0 (`self.ProjectileMovementComponent`))
  (`self.SetLifeSpan` 6.0))

(event `self.DamageComponent.OnComponentBeginOverlap`
  (params (OverlappedComponent :type "PrimitiveComponent Object Reference") (OtherActor :type "Actor Object Reference") (OtherComp :type "PrimitiveComponent Object Reference") (OtherBodyIndex :type Integer) (bFromSweep :type Boolean) (SweepResult :type "HitResult Structure (by ref)"))
  (cast `/Game/Interactive/Weapon/SheildSkill` OtherActor
    (:`then`
      (`GameplayStatics.PlaySoundAtLocation` "/Game/Sound/Monster/Healer/Heal.Heal" (`SceneComponent.K2_GetComponentLocation` (`self.CollisionComponent`)) (struct) 1.0 1.0 0.0 null null null)
      (bind _asbp_my_main_char (cast `/Game/Character/BP_MyMainChar` (`GameplayStatics.GetPlayerPawn` 0)))
      (`MyMainChar.AddEnergy` _asbp_my_main_char 5.0))
    (:`CastFailed`
      (bind _asbp_my_main_char_2 (cast `/Game/Character/BP_MyMainChar` OtherActor))
      (cast `CapsuleComponent` OtherComp)
      (`GameplayStatics.ApplyDamage` _asbp_my_main_char_2 (`self.MagicDamge`))))
  (`self.SetLifeSpan` 0.1))

(fn `UserConstructionScript`)