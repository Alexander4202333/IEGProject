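; Player character Blueprint for an action game with swappable weapons, monster-kill leveling, ability upgrades and timed enemy strengthening.
; Picked-up drops set meshes, power, attack montages, trails and skill type, while replaced weapons spawn back as drops.
; Weapon overlaps during attacks deal damage and add energy; skills branch into dash, invincible shield, double-weapon effect or magic missile.
; Damage drives hurt feedback and death, which opens an end menu or respawns the player, leaving a body.
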(event `AddKill`
  (bind _returnvalue (`self.LevelUpCondition` (`PlayerStatistic.MonsterKill` (`self.BP_PlayerStatistic`))))
  (if _returnvalue
    (`GameplayStatics.PlaySound2D` "/Game/Sound/MyMusic/LevelUp.LevelUp" 1.0 1.0 0.0 null null)
    (bind _returnvalue_2 (`|CreateWidget` "/Game/UI/Word/LevelUp.LevelUp_C"))
    (`UserWidget.AddToViewport` _returnvalue_2 0)))

(event `InputAction|Confirm`
  (params (Key :type "Key Structure"))
  ;[1 1 1] Menu
  (:`Pressed`
    (if (`self.IsOpenPickMenu`)
      (`self.PickWeapon`)
      (elif (`self.IsOpenAbilityMenu`)
        (`self.PickAbility`)))))

(event `InputAction|OpenAttributeBoard`
  (params (Key :type "Key Structure"))
  ;[1 1 1] Menu
  (:`Pressed`
    (bind _returnvalue (`|CreateWidget` "/Game/UI/PlayerUI/Attribute.Attribute_C"))
    (`UserWidget.AddToViewport` _returnvalue 0))
  (:`Released`
    (`Widget.RemoveFromParent` _returnvalue)))

(event `InputAction|OpenMenu`
  (params (Key :type "Key Structure"))
  ;[1 1 1] Menu
  (:`Pressed`
    (`self.OpenMenu` "/Game/UI/PlayerUI/Pause.Pause_C")))

(event `Guide`
  ;[1 1 1] Menu
  (`self.OpenMenu` "/Game/UI/Guide/Page.Page_C"))

(event `OpenAbilityMenu`
  (params (NewParam :type "/Game/Interactive/Ability/BPAbilityMaster Object Reference"))
  ;[1 1 1] Menu
  (set `self.IsOpenAbilityMenu` true)
  (set `self.AbilityPIck` NewParam))

(event `CloseAbilityMenu`
  ;[1 1 1] Menu
  (set `self.IsOpenAbilityMenu` false)
  (set `self.AbilityPIck` null))

(event `OpenPickMenu`
  (params (Drop :type "Actor Object Reference"))
  ;[1 1 1] Menu
  (set `self.IsOpenPickMenu` true)
  (set `self.DroptoPick` Drop))

(event `ClosePickMenu`
  ;[1 1 1] Menu
  (set `self.IsOpenPickMenu` false)
  (set `self.DroptoPick` null))

(event `DropWeapon`
  (params (SocketIndex :type Integer))
  ;[0 0.9475 1] DropWeapon
  (`StaticMeshComponent.SetStaticMesh` (select `int` SocketIndex :`0` (`self.Weapon`) :`1` (`self.Shield`) :`2` (`self.Double`)) null)
  (`|SpawnActorFromClass` (`|GetArrayItem` (`self.WeaponArray`) (`|GetArrayItem` (`self.EquipIndex`) SocketIndex)) (`KismetMathLibrary.MakeTransform` (`SceneComponent.K2_GetComponentLocation` (`self.DoubleSkillPoint`))) "Undefined" "OverrideRootScale" null null))

(event `InputAction|Skill`
  (params (Key :type "Key Structure"))
  (bind _magiceffectindex (`self.MagicEffectIndex`))
  (bind _springarm (`self.SpringArm`))
  (bind _speedupeffect (`self.SpeedUpEffect`))
  ;[1 1 1] Skill
  (:`Pressed`
    (bind _returnvalue (`self.SkillSituation`))
    (switch `int` _returnvalue
      (:`0`
        (if true
          (switch `int` (`self.SkillType`)
            (:`Default`
              ;[0 0.2224 1] SwordSkill
              (`self.BeginDash` _speedupeffect (`|GetArrayItem` (`self.MagicEffect`) (`self.SwordIndex`)))
              (`KismetSystemLibrary.Delay` 0.9)
              (`self.StopDash` _speedupeffect))
            (:`0`
              ;[0.07657 1 0] SheildSkill
              (set `self.Invinceble` true)
              (`|SpawnActorFromClass` (`|GetArrayItem` (`self.SheildSkill`) (- (`self.MagicEffectIndex`) 8)) (`KismetMathLibrary.MakeTransform` (`SceneComponent.K2_GetComponentLocation` (`self.Mesh`))) "Undefined" "OverrideRootScale" null null)
              (`KismetSystemLibrary.Delay` 1.0)
              (set `self.Invinceble` false))
            (:`1`
              ;[1 0 0.03386] DoubleSkill
              (bind _returnvalue_2 (`self.PlayAnimMontage` "/Game/Extra/Red_Knight/Animations/MonMainAtk3.MonMainAtk3"))
              (`KismetSystemLibrary.Delay` (- _returnvalue_2 0.05))
              (bind _returnvalue_3 (`|SpawnActorFromClass` "/Game/Interactive/Weapon/DoubleSkill.DoubleSkill_C" (`KismetMathLibrary.MakeTransform` (`SceneComponent.K2_GetComponentLocation` (`self.DoubleSkillPoint`))) "Undefined" "OverrideRootScale" null null))
              (`ParticleSystemComponent.SetTemplate` (`/Game/Interactive/Weapon/DoubleSkill.DoubleSkillEffect` _returnvalue_3) (`|GetArrayItem` (`self.MagicEffect`) _magiceffectindex))
              (`self.SetLifeSpan` _returnvalue_3 (* _magiceffectindex 0.18)))
            (:`2`
              ;[1 0.6431 0] MagicSkill
              (bind _returnvalue_4 (`self.PlayAnimMontage` "/Game/Extra/Red_Knight/Animations/MonMainAtk0.MonMainAtk0" 0.7))
              (`KismetSystemLibrary.Delay` (* _returnvalue_4 0.5))
              (bind _returnvalue_5 (`|SpawnActorFromClass` "/Game/Interactive/Weapon/BP_MagicMissile.BP_MagicMissile_C" (`KismetMathLibrary.MakeTransform` (`SceneComponent.GetSocketLocation` _springarm "None") (`SpringArmComponent.GetTargetRotation` _springarm)) "Undefined" "OverrideRootScale" null null))
              (bind _returnvalue_6 (`self.getMagicDamage`))
              (set `/Game/Interactive/Weapon/BP_MagicMissile.MagicDamge` _returnvalue_6 _returnvalue_5)
              (`ParticleSystemComponent.SetTemplate` (`/Game/Interactive/Weapon/BP_MagicMissile.MagicEffect` _returnvalue_5) (`|GetArrayItem` (`self.MagicEffect`) (`self.MagicEffectIndex`)))))
          (else
            (bind _returnvalue_7 (`|CreateWidget` "/Game/UI/Word/CantSkill1.CantSkill1_C"))
            (`UserWidget.AddToViewport` _returnvalue_7 0))))
      (:`1`
        (bind _returnvalue_8 (`|CreateWidget` "/Game/UI/Word/CantSkill1.CantSkill1_C"))
        (`UserWidget.AddToViewport` _returnvalue_8 0))
      (:`2`
        (bind _returnvalue_9 (`|CreateWidget` "/Game/UI/Word/CantSkill2.CantSkill2_C"))
        (`UserWidget.AddToViewport` _returnvalue_9 0)))))

(event `InputAction|Attack`
  (params (Key :type "Key Structure"))
  ;[0.5043 0 1] Attack
  (:`Pressed`
    (bind _returnvalue (`self.Attack Run` (`self.AttackIndex`)))
    (set `self.AttackIndex` _returnvalue)
    (`self.SetAttackEffect`)))

(event `InputAction|DropShield`
  (params (Key :type "Key Structure"))
  (bind _equiped (`self.Equiped`))
  ;[0 0.929 1] DropShield
  (:`Pressed`
    (if (`|GetArrayItem` _equiped 1)
      (`self.DropWeapon` 1)
      (`KismetArrayLibrary.Array_Set` _equiped 1)
      (`self.SetSkillType`))))

(event `self.ReceiveTick`
  (params (DeltaSeconds :type "Float (single-precision)")))

(event `AttackEnd`
  ;[0.5043 0 1] Attack
  (set `self.Attack` false)
  (`KismetSystemLibrary.Delay` 0.8)
  (if (not (`self.Attack`))
    (`self.ResetAttackEffect`)))

(event `self.ReceiveBeginPlay`
  (`KismetSystemLibrary.ExecuteConsoleCommand` "DisableAllScreenMessages" null)
  (if (not (`self.IsTestMap`))
    (`KismetSystemLibrary.K2_SetTimerDelegate` (delegate `addEnemyBonus`) 84.0 true))
  (`self.CreateUI`)
  ;[1 0.5134 0.0149] getHurt
  (bind _returnvalue (`|CreateWidget` "/Game/UI/PlayerUI/Hurt.Hurt_C"))
  (`UserWidget.AddToViewport` _returnvalue 0)
  (add `self.OnTakeAnyDamage` (delegate `OnTakeAnyDamage_Event_0`)))

(event `addEnemyBonus`
  ;[0 1 0.02111] MonsterLevelUp
  (set `self.EnemyBonus` (+ (`self.EnemyBonus`) 0.1))
  (bind _returnvalue (`|CreateWidget` "/Game/UI/Word/MonsterLevelUp.MonsterLevelUp_C"))
  (`UserWidget.AddToViewport` _returnvalue 0))

(event `OnTakeAnyDamage_Event_0` :!signature `self.OnTakeAnyDamage`
  (params (DamagedActor :type "Actor Object Reference") (Damage :type "Float (double-precision)") (DamageType :type "DamageType Object Reference") (InstigatedBy :type "Controller Object Reference") (DamageCauser :type "Actor Object Reference"))
  ;[1 0.5134 0.0149] getHurt
  (if (not (or (`self.Invinceble`) (`self.IsDead`)))
    (bind _returnvalue (`|CreateWidget` "/Game/UI/Word/PlayerHurtNumber.PlayerHurtNumber_C"))
    (set `/Game/UI/Word/PlayerHurtNumber.TextShow` Damage _returnvalue)
    (`UserWidget.AddToViewport` _returnvalue 0)
    (`self.SubHealth` Damage)
    (`/Game/UI/PlayerUI/Hurt.GetHurt` (stale `self.ReceiveBeginPlay` _returnvalue))
    (`PlayerCameraManager.StartCameraShake` :`self` (`GameplayStatics.GetPlayerCameraManager` 0) :`ShakeClass` "/Game/UI/PlayerUI/HurtCamaraShake.HurtCamaraShake_C")
    (if (`self.IsDead`)
      (`self.Dead`))))

(event `Dead`
  ;[1 0.5707 0] 注释
  (set `self.Attack` true)
  (bind _returnvalue (`PlayerStatistic.IsEnd` (`self.BP_PlayerStatistic`)))
  (if _returnvalue
    (`self.OpenMenu` "/Game/UI/PlayerUI/EndMenu.EndMenu_C")
    (else
      (`KismetSystemLibrary.Delay` 1.85)
      (`self.SpawnBody`)
      (`self.K2_TeleportTo` (1370.0 -440.0 -28.0))
      (`self.Revive`)
      (set `self.Attack` false))))

(event `self.DashCollsion.OnComponentBeginOverlap`
  (params (OverlappedComponent :type "PrimitiveComponent Object Reference") (OtherActor :type "Actor Object Reference") (OtherComp :type "PrimitiveComponent Object Reference") (OtherBodyIndex :type Integer) (bFromSweep :type Boolean) (SweepResult :type "HitResult Structure (by ref)"))
  ;[1 0.06785 0] CollisionDamage
  (bind _asenemy_aisword (cast `EnemyAISword` OtherActor))
  (bind _returnvalue (`self.getMagicDamage`))
  (cast `CapsuleComponent` OtherComp)
  (`GameplayStatics.ApplyDamage` _asenemy_aisword _returnvalue null self))

(event `self.Weapon.OnComponentBeginOverlap`
  (params (OverlappedComponent :type "PrimitiveComponent Object Reference") (OtherActor :type "Actor Object Reference") (OtherComp :type "PrimitiveComponent Object Reference") (OtherBodyIndex :type Integer) (bFromSweep :type Boolean) (SweepResult :type "HitResult Structure (by ref)"))
  ;[1 0.06785 0] CollisionDamage
  (if (`self.Attack`)
    (if (not (`self.IsProtect`))
      (bind _asenemy_aisword (cast `EnemyAISword` OtherActor))
      (cast `CapsuleComponent` OtherComp)
      (`self.MakeDamage` _asenemy_aisword)
      (set `self.IsProtect` true))))

(event `self.weapon.OnComponentEndOverlap`
  (params (OverlappedComponent :type "PrimitiveComponent Object Reference") (OtherActor :type "Actor Object Reference") (OtherComp :type "PrimitiveComponent Object Reference") (OtherBodyIndex :type Integer))
  ;[1 0.06785 0] CollisionDamage
  (set `self.IsProtect` false))

(event `self.Double.OnComponentBeginOverlap`
  (params (OverlappedComponent :type "PrimitiveComponent Object Reference") (OtherActor :type "Actor Object Reference") (OtherComp :type "PrimitiveComponent Object Reference") (OtherBodyIndex :type Integer) (bFromSweep :type Boolean) (SweepResult :type "HitResult Structure (by ref)"))
  ;[1 0.06785 0] CollisionDamage
  (if (`self.Attack`)
    (if (not (`self.IsProtect`))
      (bind _asenemy_aisword (cast `EnemyAISword` OtherActor))
      (cast `CapsuleComponent` OtherComp)
      (`self.MakeDamage` _asenemy_aisword)
      (set `self.IsProtect` true))))

(event `self.Double.OnComponentEndOverlap`
  (params (OverlappedComponent :type "PrimitiveComponent Object Reference") (OtherActor :type "Actor Object Reference") (OtherComp :type "PrimitiveComponent Object Reference") (OtherBodyIndex :type Integer))
  ;[1 0.06785 0] CollisionDamage
  (set `self.IsProtect` false))

(fn `Attack Run`
  (params (`Dimension 1` :type Integer))
  (returns (ReturnValue :type Integer) (ReturnValue1 :type "Float (double-precision)"))
  (locals (NewLocalVar_0 :type "Pawn Object Reference"))
  (bind _attacktype (`self.AttackType`))
  (if (not (`self.Attack`))
    (set `self.Attack` true)
    (`GameplayStatics.PlaySound2D` "/Game/Sound/MC/MainCharAttack.MainCharAttack" 1.0 1.0 0.0 null null)
    (bind _returnvalue (`self.PlayAnimMontage` (`|GetArrayItem` (`self.AttackMontages`) `Dimension 1`) (`self.AttackRate`)))
    (if (>= (`KismetMathLibrary.Conv_IntToDouble` (`self.AttackIndex`)) (`KismetMathLibrary.Conv_IntToDouble` _attacktype))
      (set `self.AttackIndex` 0)
      (else
        (bind _result (`/Engine/EditorBlueprintResources/StandardMacros.IncrementInt` `Dimension 1`)
          (:`  `
            _))))
    (return (mod _result _attacktype) _returnvalue)))

(fn `BeginDash`
  (params (self2 :type "ParticleSystemComponent Object Reference") (NewTemplate :type "ParticleSystem Object Reference"))
  (bind _charactermovement (`self.CharacterMovement`))
  (bind _camera (`self.Camera`))
  (set `CharacterMovementComponent.GroundFriction` 0.0 _charactermovement)
  (`CharacterMovementComponent.AddImpulse` _charactermovement (* (`self.GetActorForwardVector`) 2000.0) true)
  (set `CharacterMovementComponent.MaxWalkSpeed` 0.0 _charactermovement)
  (`PrimitiveComponent.SetCollisionResponseToChannel` (`self.CapsuleComponent`) "ECC_Pawn" "ECR_Overlap")
  (`PrimitiveComponent.SetCollisionEnabled` (`self.DashCollsion`) "QueryAndPhysics")
  (`CameraComponent.SetFieldOfView` _camera 112.0)
  (`CameraComponent.SetPostProcessBlendWeight` _camera 0.3)
  (`ParticleSystemComponent.SetTemplate` self2 NewTemplate)
  (`self.PlayAnimMontage` "/Game/Extra/Red_Knight/Animations/MonDash.MonDash" 0.8)
  (`GameplayStatics.PlaySound2D` "/Game/Sound/MC/Attack/launch1.launch1" 1.0 1.0 0.0 null null))

(fn `CreateUI`
  (returns (Bar :type "/Game/UI/PlayerUI/PlayerState Object Reference") (Kill :type "/Game/UI/PlayerUI/KillMosterNumber Object Reference"))
  (bind _returnvalue (`|CreateWidget` "/Game/UI/PlayerUI/Collimation.Collimation_C"))
  (set `self.Collimation` _returnvalue)
  (`UserWidget.AddToViewport` _returnvalue 0)
  (`Widget.SetVisibility` (`self.Collimation`) "Hidden")
  (bind _returnvalue_2 (`|CreateWidget` "/Game/UI/PlayerUI/PlayerState.PlayerState_C"))
  (`UserWidget.AddToViewport` _returnvalue_2 0)
  (bind _returnvalue_3 (`|CreateWidget` "/Game/UI/PlayerUI/KillMosterNumber.KillMosterNumber_C"))
  (`UserWidget.AddToViewport` _returnvalue_3 0)
  (return _returnvalue_2 _returnvalue_3))

(fn `getAttackEffect`
  (params (self2 :type "/Game/Interactive/Weapon/BPDorpMaster Object Reference"))
  (locals (Mon1 :type "Array of AnimMontage Object Reference") (Mon2 :type "Array of AnimMontage Object Reference") (Mon3 :type "Array of AnimMontage Object Reference") (Mon4 :type "Array of AnimMontage Object Reference") (Mon5 :type "Array of AnimMontage Object Reference") (Mon6 :type "Array of AnimMontage Object Reference") (Mon7 :type "Array of AnimMontage Object Reference") (Mon0 :type "Array of AnimMontage Object Reference"))
  (bind _weaponindex (`/Game/Interactive/Weapon/BPDorpMaster.WeaponIndex` self2))
  (if (or (< _weaponindex 8) (> _weaponindex 11))
    (switch `int` _weaponindex
      (:`Default`
        (set `self.AttackEffect` 0)
        (set `self.AttackMontages` (`local.Mon3`) :!label _label))
      (:`0`
        (set `self.AttackEffect` 0)
        (set `self.AttackMontages` (`local.Mon0`) :!label _label_2))
      (:`1`
        (set `self.AttackMontages` (`local.Mon1`))
        (set `self.AttackEffect` 0 :!label _label_3))
      (:`2`
        (set `self.AttackMontages` (`local.Mon2`))
        (goto _label_3))
      (:`3`
        (set `self.AttackEffect` 1)
        (goto _label))
      (:`4`
        (goto _label_2))
      (:`5`
        (set `self.AttackEffect` 2)
        (goto _label))
      (:`6`
        (set `self.AttackEffect` 3)
        (goto _label))
      (:`7`
        (set `self.AttackEffect` 4)
        (goto _label)))
    (return)))

(fn `MakeDamage`
  (params (DamagedActor :type "Actor Object Reference"))
  (if (and (!= DamagedActor self) (`self.Attack`))
    (bind _returnvalue (`self.getAttackDamage`))
    (`GameplayStatics.ApplyDamage` DamagedActor _returnvalue null self)
    (`self.AddEnergy` 10.0)))

(fn `OpenMenu`
  (params (Class :type "UserWidget Class Reference"))
  (bind _returnvalue (`GameplayStatics.GetPlayerController` 0))
  ;[0 1 0.9618] OpenMenu
  (set `PlayerController.bShowMouseCursor` true _returnvalue)
  (bind _returnvalue_2 (`|CreateWidget` Class))
  (`UserWidget.AddToViewport` _returnvalue_2 0)
  (`WidgetBlueprintLibrary.SetInputMode_UIOnlyEx` _returnvalue _returnvalue_2)
  (`GameplayStatics.SetGamePaused` true))

(fn `PickAbility`
  (bind _abilitypick (`self.AbilityPIck`))
  (`/Engine/EditorBlueprintResources/StandardMacros.IsValid` _abilitypick
    (:`Is Valid`
      (bind _asbpability_master (cast `/Game/Interactive/Ability/BPAbilityMaster` _abilitypick))
      (bind _returnvalue (`self.ConsumePoint`))
      (if _returnvalue
        (bind _returnvalue_2 (`|CreateWidget` "/Game/UI/Word/AbilitySucceed.AbilitySucceed_C"))
        (`UserWidget.AddToViewport` _returnvalue_2 0)
        (`GameplayStatics.PlaySound2D` "/Game/Sound/MyMusic/PickAbilitySound.PickAbilitySound" 1.0 1.0 0.0 null null)
        (switch `int` (`/Game/Interactive/Ability/BPAbilityMaster.AbilityIndex` _asbpability_master)
          (:`0`
            (`self.addAttackBonus` 0.1))
          (:`1`
            (`self.addMagicBonus` 0.1))
          (:`2`
            (`self.addMaxHealth` 25.0))
          (:`3`
            (`self.addMaxEnergy` 15.0))
          (:`4`
            (`self.addSpeed` 25.0)))
        (else
          (bind _returnvalue_3 (`|CreateWidget` "/Game/UI/Word/AbilityFail.AbilityFail_C"))
          (`UserWidget.AddToViewport` _returnvalue_3 0))))))

(fn `PickWeapon`
  (bind _droptopick (`self.DroptoPick`))
  (bind _collimation (`self.Collimation`))
  (`/Engine/EditorBlueprintResources/StandardMacros.IsValid` _droptopick
    (:`Is Valid`
      (bind _asbpdorp_master (cast `/Game/Interactive/Weapon/BPDorpMaster` _droptopick))
      (if (> (`/Game/Interactive/Weapon/BPDorpMaster.WeaponLevel` _asbpdorp_master) (`self.Level`))
        (bind _returnvalue (`|CreateWidget` "/Game/UI/Word/WeaponFail.WeaponFail_C"))
        (`UserWidget.AddToViewport` _returnvalue 0)
        (else
          (`GameplayStatics.PlaySound2D` "/Game/Sound/MyMusic/PickAbilitySound.PickAbilitySound" 1.0 1.0 0.0 null null)
          (`self.getAttackEffect` _asbpdorp_master)
          (bind _socketindex (`/Game/Interactive/Weapon/BPDorpMaster.SocketIndex` _asbpdorp_master))
          (bind _returnvalue_2 (`self.GetPickSituation` _socketindex))
          (switch `int` _returnvalue_2
            (:`0`
              (`self.DropWeapon` 1)
              (`self.DropWeapon` 0))
            (:`1`
              (`self.DropWeapon` 2))
            (:`2`
              (`self.DropWeapon` _socketindex))
            (:`3`
              _))
          (`StaticMeshComponent.SetStaticMesh` (select `int` _socketindex :`0` (`self.Weapon`) :`1` (`self.Shield`) :`2` (`self.Double`)) (`/Game/Interactive/Weapon/BPDorpMaster.WeaponMesh` _asbpdorp_master))
          (if (!= _socketindex 1)
            (set `self.AttackPower` (`/Game/Interactive/Weapon/BPDorpMaster.Damage` _asbpdorp_master))
            (set `self.MagicPower` (`/Game/Interactive/Weapon/BPDorpMaster.MagicDamge` _asbpdorp_master))
            (if (== _socketindex 0)
              (bind _weaponindex (`/Game/Interactive/Weapon/BPDorpMaster.WeaponIndex` _asbpdorp_master))
              (set `self.SwordIndex` _weaponindex)
              (else
                (set `self.SwordIndex` 0)
                (set `self.MagicEffectIndex` _weaponindex :!label _label)))
            (else
              (goto _label)))
          (bind _output_get (set `self.IsMagic` (`/Game/Interactive/Weapon/BPDorpMaster.Magic` _asbpdorp_master)))
          (if _output_get
            (`Widget.SetVisibility` _collimation "Visible")
            (else
              (`Widget.SetVisibility` _collimation "Hidden")))
          (`KismetArrayLibrary.Array_Set` (`self.EquipIndex`) _socketindex _weaponindex)
          (`self.SetSkillType`)
          (set `self.AttackIndex` 0)
          (`self.K2_DestroyActor` (`self.DroptoPick`))
          (`self.ClosePickMenu`)
          (`self.ResetAttack`))))))

(fn `ResetAttackEffect`
  (`SceneComponent.SetVisibility` (`self.Tail`) false false)
  (`SceneComponent.SetVisibility` (`self.DoubleTrail6`) false false)
  (`SceneComponent.SetVisibility` (`self.DoubleTrail7`) false false)
  (`SceneComponent.SetVisibility` (`self.DoubleTrail5`) false false))

(fn `SetAttackEffect`
  (bind _equiped (`self.Equiped`))
  (switch `int` (`self.AttackEffect`)
    (:`1`
      (if (`|GetArrayItem` _equiped)
        (`SceneComponent.SetVisibility` (`self.Tail`) true false)))
    (:`2`
      (if (`|GetArrayItem` _equiped 2)
        (`SceneComponent.SetVisibility` (`self.DoubleTrail5`) true false)))
    (:`3`
      (if true
        (`SceneComponent.SetVisibility` (`self.DoubleTrail6`) true false)))
    (:`4`
      (if true
        (`SceneComponent.SetVisibility` (`self.DoubleTrail7`) true false)))))

(fn `SpawnBody`
  (bind _mesh (`self.Mesh`))
  (bind _returnvalue (`|SpawnActorFromClass` "/Game/Maps/Meshes/MainCharBody.MainCharBody_C" (`SceneComponent.K2_GetComponentToWorld` _mesh) "Undefined" "OverrideRootScale" null null))
  (`SkinnedMeshComponent.SetSkinnedAssetAndUpdate` (`Character.Mesh` _returnvalue) (`SkinnedMeshComponent.SkeletalMesh` _mesh) true))

(fn `StopDash`
  (params (self2 :type "ParticleSystemComponent Object Reference"))
  (bind _charactermovement (`self.CharacterMovement`))
  (bind _camera (`self.Camera`))
  (`ParticleSystemComponent.SetTemplate` self2 null)
  (`PrimitiveComponent.SetCollisionEnabled` (`self.DashCollsion`) "NoCollision")
  (`PrimitiveComponent.SetCollisionResponseToChannel` (`self.CapsuleComponent`) "ECC_Pawn" "ECR_Block")
  (`CameraComponent.SetPostProcessBlendWeight` _camera 0.0)
  (`CameraComponent.SetFieldOfView` _camera 105.0)
  (set `CharacterMovementComponent.GroundFriction` 8.0 _charactermovement)
  (set `CharacterMovementComponent.MaxWalkSpeed` (`self.Speed`) _charactermovement))

(fn `UserConstructionScript`
  (set `self.MaxHealth` 180.0))